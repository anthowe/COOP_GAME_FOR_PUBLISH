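; BP_EnemyPortal is an enemy spawn point that creates BP_AdvancedAI pawns at its SpawnBox location.
; Its Easy and Medium events each spawn one pawn, provided fewer than 100 BP_AdvancedAI actors exist in the world.
; Both events run identical logic, and nothing in this graph calls them.
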(event `Easy`
  (bind _outactors (`GameplayStatics.GetAllActorsOfClass` "/Game/AdvancedAI/BP_AdvancedAI.BP_AdvancedAI_C"))
  (if (< (`KismetArrayLibrary.Array_Length` _outactors) 100)
    (`AIBlueprintHelperLibrary.SpawnAIFromClass` "/Game/AdvancedAI/BP_AdvancedAI.BP_AdvancedAI_C" null (`SceneComponent.K2_GetComponentLocation` (`self.SpawnBox`)))))

(event `Medium`
  (bind _outactors (`GameplayStatics.GetAllActorsOfClass` "/Game/AdvancedAI/BP_AdvancedAI.BP_AdvancedAI_C"))
  (if (< (`KismetArrayLibrary.Array_Length` _outactors) 100)
    (`AIBlueprintHelperLibrary.SpawnAIFromClass` "/Game/AdvancedAI/BP_AdvancedAI.BP_AdvancedAI_C" null (`SceneComponent.K2_GetComponentLocation` (`self.SpawnBox`)))))

(fn `UserConstructionScript`)