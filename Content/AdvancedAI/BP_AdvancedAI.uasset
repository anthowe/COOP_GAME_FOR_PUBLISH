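; BP_AdvancedAI is an AI-controlled actor with health that takes damage and is removed after death.
; On BeginPlay its AI controller runs the BT_AdvancedAI behavior tree.
; Damage events update and print Health; radial damage subtracts correctly, while AnyDamage reverses the subtraction to Damage minus Health.
; Tick polls for depleted Health and destroys the actor after a delay; the rifle cleanup logic is unconnected.
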(event `self.ReceiveBeginPlay`
  (`AIController.RunBehaviorTree` (`AIBlueprintHelperLibrary.GetAIController` self) "/Game/AdvancedAI/AI/BT_AdvancedAI.BT_AdvancedAI"))

(event `self.ReceiveAnyDamage`
  (params (Damage :type "Float (single-precision)") (DamageType :type "DamageType Object Reference") (InstigatedBy :type "Controller Object Reference") (DamageCauser :type "Actor Object Reference"))
  (bind _output_get (set `self.Health` (- Damage (`self.Health`))))
  (`KismetSystemLibrary.PrintString` (`KismetStringLibrary.Concat_StrStr` "Health" (`KismetStringLibrary.Conv_DoubleToString` _output_get))))

(event `self.ReceiveRadialDamage`
  (params (DamageReceived :type "Float (single-precision)") (DamageType :type "DamageType Object Reference") (Origin :type "Vector Structure") (HitInfo :type "HitResult Structure (by ref)") (InstigatedBy :type "Controller Object Reference") (DamageCauser :type "Actor Object Reference"))
  (bind _output_get (set `self.Health` (- (`self.Health`) DamageReceived)))
  (`KismetSystemLibrary.PrintString` (`KismetStringLibrary.Concat_StrStr` "Health" (`KismetStringLibrary.Conv_DoubleToString` _output_get) "" (`KismetStringLibrary.Conv_VectorToString` Origin)) true true (struct :`R` 1.0 :`G` 0.935816 :`A` 1.0) 10.0))

(event `self.ReceiveTick`
  (params (DeltaSeconds :type "Float (single-precision)"))
  (if (<= (`self.Health`) 0.0)
    (`KismetSystemLibrary.Delay` 5.0)
    (`self.K2_DestroyActor`)))

(fn `UserConstructionScript`)