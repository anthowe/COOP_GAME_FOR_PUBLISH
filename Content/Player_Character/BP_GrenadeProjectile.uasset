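; Grenade projectile that explodes on a short fuse started at BeginPlay, regardless of impact.
; Explode spawns a particle effect, deals full radial damage credited to the instigator, destroys the actor and draws a debug sphere of the damage radius.
; Left mouse press also calls ExplodeProjectile, which is not defined in these graphs.
; The Hit event is empty, and an alternate BP_Explosion-spawning path is left disconnected.
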(event `self.ReceiveHit`
  (params (MyComp :type "PrimitiveComponent Object Reference") (Other :type "Actor Object Reference") (OtherComp :type "PrimitiveComponent Object Reference") (bSelfMoved :type Boolean) (HitLocation :type "Vector Structure") (HitNormal :type "Vector Structure") (NormalImpulse :type "Vector Structure") (Hit :type "HitResult Structure (by ref)"))
  ;[1 1 1] Event Hit did not work
)

(event `self.ReceiveBeginPlay`
  (`KismetSystemLibrary.Delay` 0.3)
  (`self.Explode`))

(event `Key|LeftMouseButton`
  (params (Key :type "Key Structure"))
  (:`Pressed`
    ;[1 1 1] BP Version that works will disconnect while testing
    (`self.ExplodeProjectile`)))

(event `Explode`
  (bind _returnvalue (`self.K2_GetActorLocation`))
  ;[1 1 1] BP Version that works will disconnect while testing
  (`GameplayStatics.SpawnEmitterAtLocation` "/Game/Weapons/WeaponEffects/Explosion/P_Explosion.P_Explosion" _returnvalue)
  (`GameplayStatics.ApplyRadialDamage` :`BaseDamage` 250.0 :`Origin` _returnvalue :`DamageRadius` (`self.Damage Radius`) :`DamageCauser` self :`InstigatedByController` (`self.GetInstigatorController`) :`bDoFullDamage` true)
  (`self.K2_DestroyActor`)
  (`KismetSystemLibrary.DrawDebugSphere` _returnvalue (`self.Damage Radius`) 12 (struct :`R` 1.0 :`G` 0.837795 :`A` 1.0) 1.0 1.0))

(fn `UserConstructionScript`)