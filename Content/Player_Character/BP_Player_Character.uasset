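; Player character Blueprint that sets up the local player's HUD and makes noise when landing.
; On BeginPlay, only if locally controlled, it creates crosshair and health indicator widgets and adds them to the viewport.
; Landing reports a noise event at the actor's location with itself as instigator.
; An unconnected debug snippet line-traces from the camera and prints the hit actor's name, but never runs.
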(event `self.ReceiveBeginPlay`
  (if (`self.IsLocallyControlled`)
    (`|ExecutionSequence`
      (:`then_0`
        (bind _returnvalue (`|CreateWidget` "/Game/MenuSystem/WBP_Crosshair.WBP_Crosshair_C"))
        (`UserWidget.AddToViewport` _returnvalue 0))
      (:`then_1`
        (bind _returnvalue_2 (`|CreateWidget` "/Game/MenuSystem/WBP_HealthIndicator.WBP_HealthIndicator_C"))
        (`UserWidget.AddToViewport` _returnvalue_2 0)))))

(event `self.OnLanded`
  (params (Hit :type "HitResult Structure (by ref)"))
  (`AISense_Hearing.ReportNoiseEvent` (`self.K2_GetActorLocation`) 1.0 self))

(event `Key|LeftMouseButton`
  (params (Key :type "Key Structure"))
  ;[1 1 1] BP for linetrace identify
)

(fn `UserConstructionScript`)